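; BP_PuzzleGate is a puzzle gate whose door opens once enough items have been collected.
; CollectItem increments a counter and, on reaching the required count, fires a DoOnce that calls OpenDoor and plays a 2D door sound.
; OpenDoor plays a timeline that drives the door's relative location from its DoorUp track.
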(event Custom|Open%20Door
  (bind _door_up (Timeline|Open%20Door%20Anim Play)
    (:Update
      (Transformation|SetRelativeLocation (Variables|Default|GetDoor) _door_up false false))))

(event Custom|Collect%20Item
  (Math|Integer|IncrementInt (Variables|Default|GetcurrentItemsCollected)
    (:%20%20
      (if (>= (Variables|Default|GetcurrentItemsCollected) (Variables|Default|GetmaxtItemsCollected))
        (Utilities|FlowControl|DoOnce false
          (:Completed
            (CallFunction|OpenDoor)
            (Audio|PlaySound2D "/Game/SE_Door.SE_Door" 1.0 1.0 0.0 0 0)))))))

(fn ConstructionScript)